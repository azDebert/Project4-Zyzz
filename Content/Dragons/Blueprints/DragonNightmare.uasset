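; DragonNightmare is a dragon enemy with health, a hand melee attack montage and a death sequence.
; It registers itself with a DragonHealthBar widget as the health source, shown only while a PlayerWizard overlaps SphereHealth.
; Separate events handle AOE damage, which clamps Health, and other damage, which does not.
; At zero health both paths detach the controller, play the death animation and destroy the actor after a delay.
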(event OnComponentBeginOverlap(SphereHealth)
  (params (OverlappedComponent :type Primitive%20Component%20Object%20Reference) (OtherActor :type Actor%20Object%20Reference) (OtherComp :type Primitive%20Component%20Object%20Reference) (OtherBodyIndex :type Integer) (bFromSweep :type Boolean) (SweepResult :type Hit%20Result%20Structure%20%28by%20ref%29))
  ;[1 1 1] If player is in a certain range of the dragon, Dragon's health becomes visible
  (Utilities|Casting|CastToPlayerWizard OtherActor)
  (Rendering|SetVisibility (Variables|Default|GetWidget) true false))

(event OnComponentEndOverlap(SphereHealth)
  (params (OverlappedComponent :type Primitive%20Component%20Object%20Reference) (OtherActor :type Actor%20Object%20Reference) (OtherComp :type Primitive%20Component%20Object%20Reference) (OtherBodyIndex :type Integer))
  ;[1 1 1] If player is in a certain range of the dragon, Dragon's health becomes visible
  (Utilities|Casting|CastToPlayerWizard OtherActor)
  (Rendering|SetVisibility (Variables|Default|GetWidget) false false))

(event EventBeginPlay
  ;[1 1 1] Links HealthBar to health
  (Utilities|FlowControl|Sequence
    (:then_0
      (Variables|Default|SetHealth (Variables|Default|GetMaxHealth))
      (bind _asdragon_health_bar (Utilities|Casting|CastToDragonHealthBar (UserInterface|GetUserWidgetObject (Variables|Default|GetWidget))))
      (Variables|/Game/HUD/DragonHealthBar.DragonHealthBar_C|SetHealthInterface _asdragon_health_bar self))
    (:then_1
      (Physics|SetSimulatePhysics (Variables|Collision|GetCapsuleComponent) false))))

(event EventMeleeAttack
  (Animation|Montage|PlayMontage (Variables|Character|GetMesh) "/Game/Dragons/Animations/DragonTheNightmare/AttackHandAnim_Montage.AttackHandAnim_Montage"))

(event EventDamage
  (params (Amount :type Float%20%28single-precision%29))
  ;[1 1 1] Updates Health if AOE damage affects it
  (Variables|Default|SetHealth (Math|Float|Clamp(Float) (- (Variables|Default|GetHealth) Amount) 0.0 (Variables|Default|GetMaxHealth)))
  (if (<= (Variables|Default|GetHealth) 0.0)
    ;[1 1 1] Prepares for Dragons Death
    (Class|Pawn|DetachfromControllerPendingDestroy)
    (Components|Animation|PlayAnimation (Variables|Character|GetMesh) "/Game/Dragons/Animations/DragonTheNightmare/DieAnim.DieAnim" false)
    (Utilities|FlowControl|Delay 3.0)
    (Actor|DestroyActor)))

(event Game|Damage|EventAnyDamage
  (params (Damage :type Float%20%28single-precision%29) (DamageType :type Damage%20Type%20Object%20Reference) (InstigatedBy :type Controller%20Object%20Reference) (DamageCauser :type Actor%20Object%20Reference))
  ;[1 1 1] Updates Health if any damage besides aoe affects it
  (Variables|Default|SetHealth (- (Variables|Default|GetHealth) Damage))
  (if (<= (Variables|Default|GetHealth) 0.0)
    ;[1 1 1] Prepares for Dragons Death
    (Class|Pawn|DetachfromControllerPendingDestroy)
    (Components|Animation|PlayAnimation (Variables|Character|GetMesh) "/Game/Dragons/Animations/DragonTheNightmare/DieAnim.DieAnim" false)
    (Utilities|FlowControl|Delay 3.0)
    (Actor|DestroyActor)))

(fn ConstructionScript)

(fn GetHealthasRation
  (return (/ (Variables|Default|GetHealth) (Variables|Default|GetMaxHealth))))